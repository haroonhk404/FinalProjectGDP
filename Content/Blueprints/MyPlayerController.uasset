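; Player controller Blueprint holding disconnected logic for respawning the first-person player at the game mode's checkpoint.
; One chain casts the game mode to BP_FirstPersonGameMode; another teleports the existing character slightly above the checkpoint with its rotation, or spawns and possesses a new BP_FirstPersonCharacter there.
; Neither chain is wired to an event, so none of it runs, and the construction script is empty.
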(fn `UserConstructionScript`)